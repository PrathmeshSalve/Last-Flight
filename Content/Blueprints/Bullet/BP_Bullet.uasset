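; BP_Bullet is a projectile actor that quits the game when it hits its TargetPawn.
; On BeginPlay it binds to its own OnActorHit and passes each hit to HandleOnHit.
; That function spawns the NS_BulletBurst Niagara effect at the impact point, aligned to the surface normal, then quits if the hit actor is the target, otherwise destroys the bullet.
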(event `self.ReceiveBeginPlay`
  (add `self.OnActorHit` (delegate `OnComponentHit`)))

(event `OnComponentHit` :!signature `self.OnActorHit`
  (params (SelfActor :type "Actor Object Reference") (OtherActor :type "Actor Object Reference") (NormalImpulse :type "Vector Structure") (Hit :type "HitResult Structure (by ref)"))
  (`self.HandleOnHit` OtherActor Hit))

(fn `HandleOnHit`
  (params (OtherActor :type "Object Object Reference") (Hit :type "HitResult Structure (by ref)"))
  (bind (_bblockinghit _binitialoverlap _time _distance _location _impactpoint _normal) (`GameplayStatics.BreakHitResult` Hit))
  (`NiagaraFunctionLibrary.SpawnSystemAtLocation` "/Game/Assets/FX/NS_BulletBurst.NS_BulletBurst" _location (`KismetMathLibrary.Conv_VectorToRotator` _normal))
  (if (== (`local.OtherActor`) (`self.TargetPawn`))
    (`KismetSystemLibrary.QuitGame` null "Quit")
    (else
      (`self.K2_DestroyActor`))))

(fn `UserConstructionScript`)